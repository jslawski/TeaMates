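; Delivery zone for a tea order, hidden at start with a random required amount, completed when an overlapping actor carries enough of the matching tea type.
; SetupDeliveryZoneVisuals picks the tea's drop mesh, shows the username and starts a random expiry timer, displayed as a countdown on Tick.
; Delivery or expiry hides the zone, plays a sound and broadcasts the order result to all actors implementing the BP_OrderComplete interface.
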(event Custom|OrderExpired
  (CallFunction|ExpireOrder true))

(event EventBeginPlay
  (Rendering|SetActorHiddenInGame true)
  (Collision|SetActorEnableCollision false)
  (bind _output_get (Variables|Default|SetDeliveryThreshold (Math|Random|RandomIntegerinRange 7 15)))
  (Rendering|Components|TextRender|SetText (Variables|Default|GetThreshold) (Utilities|Text|ToText(Integer) _output_get)))

(event Collision|EventActorBeginOverlap
  (params (OtherActor :type Actor%20Object%20Reference))
  (bind _totaltea (Class|BPTeaHolderInterface|GetTotalTea(Message) OtherActor))
  (bind _teatype (Class|BPTeaTypeInterface|GetTeaType(Message) OtherActor))
  (if (and (>= _totaltea (Variables|Default|GetDeliveryThreshold)) (== (Variables|Default|GetTeaType) _teatype))
    (Class|BPTeaHolderInterface|RemoveTea(Message) OtherActor)
    (Rendering|SetActorHiddenInGame true)
    (Collision|SetActorEnableCollision false)
    (Utilities|Time|ClearTimerbyFunctionName 0 "ExpireOrder")
    (Audio|PlaySound2D "/Game/Audio/Delivery_Successful.Delivery_Successful" 1.0 1.0 0.0 0 0)
    (Development|PrintString "Order Completed!!")
    (CallFunction|OnOrderComplete false)))

(event EventTick
  (params (DeltaSeconds :type Float%20%28single-precision%29))
  (bind _ordertimer (Variables|Default|GetOrderTimer))
  (bind _returnvalue (Utilities|Time|GetTimerRemainingTimebyHandle _ordertimer))
  (if (> _returnvalue 0.0)
    (Rendering|Components|TextRender|SetText (Variables|Default|GetTimeRemaining) (Utilities|Text|ToText(Float) (Math|Conversions|ToFloat(Integer) (Math|Float|Round _returnvalue)) "HalfToEven"))))

(fn ConstructionScript)

(fn ExpireOrder
  (params (missed :type Boolean))
  (Development|PrintString "Order Expired!")
  (Rendering|SetActorHiddenInGame true)
  (Collision|SetActorEnableCollision false)
  (Audio|PlaySound2D "/Game/Audio/Delivery_Failed.Delivery_Failed" 1.0 1.0 0.0 0 0)
  (CallFunction|OnOrderComplete true))

(fn OnOrderComplete
  (params (Expired :type Boolean))
  (bind _structout (Utilities|Struct|SetmembersinOrderInfo (Variables|Default|GetcurrentOrder) Expired))
  (bind _outactors (Actor|GetAllActorswithInterface "/Game/Blueprints/BP_OrderComplete.BP_OrderComplete_C"))
  (for _array_element _outactors
    (Class|BPOrderComplete|OnOrderComplete(Message) _array_element _structout)))

(fn GetTeaMenu
  (return 0))

(fn GetTeaType
  (return (Variables|Default|GetTeaType)))

(fn SetTeaType
  (params (TeaType :type Integer))
  (bind _output_get (Variables|Default|SetTeaType TeaType))
  (return _output_get))

(fn SetupDeliveryZoneVisuals
  (params (TeaType :type Integer) (Username :type String))
  (bind _staticmesh1 (Variables|Default|GetStaticMesh1))
  (switch int TeaType
    (:0
      (Components|StaticMesh|SetStaticMesh _staticmesh1 "/Game/TeaTypes/BlackTea_Drop.BlackTea_Drop"))
    (:1
      (Components|StaticMesh|SetStaticMesh _staticmesh1 "/Game/TeaTypes/BlueTea_Drop.BlueTea_Drop"))
    (:2
      (Components|StaticMesh|SetStaticMesh _staticmesh1 "/Game/TeaTypes/GreenTea_Drop.GreenTea_Drop"))
    (:3
      (Components|StaticMesh|SetStaticMesh _staticmesh1 "/Game/TeaTypes/LemonTea_Drop.LemonTea_Drop")))
  (Rendering|Components|TextRender|SetText (Variables|Default|GetUsername) (Utilities|Text|ToText(String) Username))
  (bind _returnvalue (Utilities|Time|SetTimerbyEvent (EventDispatchers|CreateEvent :!event Custom|OrderExpired) (Math|Random|RandomFloatinRange (Variables|Default|GetMinTimeToExpire) (Variables|Default|GetMaxTimetoExpire))))
  (Variables|Default|SetOrderTimer _returnvalue)
  (return (.ReturnValue (Utilities|Map|Find (Variables|Default|GetTeaMenu) TeaType))))