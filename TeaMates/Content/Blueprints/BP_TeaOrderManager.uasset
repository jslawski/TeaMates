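; Manager actor that turns Twitch chat commands into tea orders and spawns for a tea delivery game.
; On BeginPlay it gathers delivery zones and flying-thing spawners, then binds "order" and "spawn" commands through the game instance's connection.
; Orders activate the first zone with collision disabled, while a looping timer adds random default orders the same way.
; Spawn creates a named tea pickup, or triggers a random spawner for "knife".
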(event Custom|OrderPlaced
  (params (Parameters :type Array%20of%20Strings) (Sender :type Twitch%20Message%20Author%20Structure))
  (bind _returnvalue (Utilities|String|JoinStringArray Parameters " "))
  (bind _teamenu (Variables|Default|GetTeaMenu))
  (bind (_value _returnvalue_2) (Utilities|Map|Find _teamenu _returnvalue))
  (if _returnvalue_2
    (bind _index (Utilities|FlowControl|ForLoopwithBreak 0 (Utilities|Array|Length (Variables|Default|GetOut%20Actors)) :!label _label)
      (:LoopBody
        (if (not (Class|PrimitiveComponent|IsCollisionEnabled (Variables|/Game/Blueprints/BP_DeliveryZone.BP_DeliveryZone_C|GetBox (Utilities|Array|Get(acopy) (Variables|Default|GetOut%20Actors) _index))))
          (CallFunction|SetupDeliveryZone (Utilities|Array|Get(acopy) (Variables|Default|GetOut%20Actors) _index) _value (.DisplayName (Utilities|Struct|BreakTwitchMessageAuthor Sender)))
          (goto _label Break))))))

(event Custom|SpawnObject
  (params (Parameters :type Array%20of%20Strings) (Sender :type Twitch%20Message%20Author%20Structure))
  (bind _displayname (Utilities|Struct|BreakTwitchMessageAuthor Sender))
  (bind _returnvalue (Utilities|String|JoinStringArray Parameters " "))
  (bind _teamenu (Variables|Default|GetTeaMenu))
  (bind (_value _returnvalue_2) (Utilities|Map|Find _teamenu _returnvalue))
  (if _returnvalue_2
    (bind _returnvalue_3 (Game|SpawnActorfromClass "/Game/Blueprints/BP_TeaPickup.BP_TeaPickup_C" (Math|Transform|MakeTransform (Math|Vector|MakeVector (Math|Random|RandomFloatinRange -1e+03 1e+03) -6e+02 1e+02)) "Undefined" 0 0))
    (Default|SetSpecificTea _returnvalue_3 _displayname _value)
    (elif (Utilities|Enum|Equal(Enum) _returnvalue "knife")
      (Default|Spawn (Utilities|Array|Get(acopy) (Variables|Default|GetObstacleSpawnLocations) (Math|Random|RandomInteger 2)) _displayname))))

(event EventBeginPlay
  (bind _outactors (Actor|GetAllActorsOfClass "/Game/Blueprints/BP_DeliveryZone.BP_DeliveryZone_C"))
  (bind _outactors_2 (Actor|GetAllActorsOfClass "/Game/Blueprints/BP_DeliveryZoneFlipped.BP_DeliveryZoneFlipped_C"))
  (Utilities|Array|AppendArray _outactors _outactors_2)
  (Variables|Default|SetOut%20Actors _outactors)
  (bind _outactors_3 (Actor|GetAllActorsOfClass "/Game/Blueprints/BP_DirectionalFlyingThingsSpawner.BP_DirectionalFlyingThingsSpawner_C"))
  (Variables|Default|SetObstacleSpawnLocations _outactors_3)
  (Utilities|Time|SetTimerbyFunctionName 0 "PlaceDefaultOrder" 2e+01 true)
  (bind _asteamates_game_instance (Utilities|Casting|CastToteamatesGameInstance (Game|GetGameInstance)))
  (bind _connection (Default|GetConnection _asteamates_game_instance))
  (Class|TwitchPluginBPLibrary|CreateTwitchCommand _connection (Utilities|Struct|MakeTwitchCommandBinding (Utilities|Struct|MakeTwitchCommand "order" "Put in an order for tea" (Utilities|Array|MakeArray "") false) (EventDispatchers|CreateEvent :!event Custom|OrderPlaced)))
  (bind _asteamates_game_instance_2 (Utilities|Casting|CastToteamatesGameInstance (Game|GetGameInstance)))
  (bind _connection_2 (Default|GetConnection _asteamates_game_instance_2))
  (bind _returnvalue (Class|TwitchPluginBPLibrary|CreateTwitchCommand _connection_2 (Utilities|Struct|MakeTwitchCommandBinding (Utilities|Struct|MakeTwitchCommand "spawn" "Spawn tea bubble" (Utilities|Array|MakeArray "") false) (EventDispatchers|CreateEvent :!event Custom|SpawnObject))))
  (Development|PrintString (Utilities|String|Append "Bind Success? " (Utilities|String|ToString(Boolean) _returnvalue))))

(event EventTick
  (params (DeltaSeconds :type Float%20%28single-precision%29)))

(fn ConstructionScript)

(fn BPTwitchAutoGenFunc
  (params (Parameters :type Array%20of%20Strings) (Sender :type Twitch%20Message%20Author%20Structure))
  (return))

(fn SetupDeliveryZone
  (params (DeliveryZoneActor :type Actor%20Object%20Reference) (TeaType :type Integer) (Username :type String))
  (Rendering|SetActorHiddenInGame DeliveryZoneActor false)
  (Collision|SetActorEnableCollision DeliveryZoneActor true)
  (Class|BPTeaTypeInterface|SetTeaType(Message) DeliveryZoneActor TeaType)
  (Class|BPDeliveryZoneInterface|SetupDeliveryZoneVisuals(Message) DeliveryZoneActor TeaType Username))

(fn PlaceDefaultOrder
  (bind _index (Utilities|FlowControl|ForLoopwithBreak 0 (Utilities|Array|Length (Variables|Default|GetOut%20Actors)) :!label _label)
    (:LoopBody
      (if (not (Class|PrimitiveComponent|IsCollisionEnabled (Variables|/Game/Blueprints/BP_DeliveryZone.BP_DeliveryZone_C|GetBox (Utilities|Array|Get(acopy) (Variables|Default|GetOut%20Actors) _index))))
        (CallFunction|SetupDeliveryZone (Utilities|Array|Get(acopy) (Variables|Default|GetOut%20Actors) _index) (Math|Random|RandomInteger 4) (Utilities|Array|Get(acopy) (Variables|Default|GetDefaultNames) (Math|Random|RandomInteger 8)))
        (goto _label Break)))))