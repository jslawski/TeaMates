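; BP_MovingObstacle is an obstacle actor that moves along negative world X.
; Every Tick it overwrites the static mesh's physics linear velocity with that direction scaled by Speed.
; Speed is copied from the BP_Constants actor only on actor begin overlap, as BeginPlay is empty.
; The mesh's own begin-overlap event just prints a debug message.
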(event OnComponentBeginOverlap(StaticMeshComponent)
  (params (OverlappedComponent :type Primitive%20Component%20Object%20Reference) (OtherActor :type Actor%20Object%20Reference) (OtherComp :type Primitive%20Component%20Object%20Reference) (OtherBodyIndex :type Integer) (bFromSweep :type Boolean) (SweepResult :type Hit%20Result%20Structure%20%28by%20ref%29))
  (Development|PrintString "Overlap!!"))

(event EventBeginPlay)

(event Collision|EventActorBeginOverlap
  (params (OtherActor :type Actor%20Object%20Reference))
  (bind _returnvalue (Actor|GetActorOfClass "/Game/Blueprints/BP_Constants.BP_Constants_C"))
  (Variables|Default|SetSpeed (Variables|/Game/Blueprints/BP_Constants.BP_Constants_C|GetSpeed _returnvalue)))

(event EventTick
  (params (DeltaSeconds :type Float%20%28single-precision%29))
  (Physics|SetPhysicsLinearVelocity (Variables|Debug|GetStaticMeshComponent) (* (Math|Vector|MakeVector -1.0 0.0 0.0) (Variables|Default|GetSpeed)) false "None"))

(fn ConstructionScript)