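; Player controller for a two-character tea game (TeaMates), driving both the pot and the cup from one set of input bindings.
; BeginPlay spawns a cup controller and cup, links them by possession, and plays the theme song.
; Pot axes move the controlled pawn and Cup axes move the spawned cup, along delta-scaled vectors rebuilt each Tick.
; It also handles game restart and quit, and offers a ReduceHealth function.
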(event EventBeginPlay
  (bind _returnvalue (Math|Transform|MakeTransform "0.000000,400.000000,64.000000"))
  (bind _returnvalue_2 (Game|SpawnActorfromClass "/Game/Blueprints/BP_CupController.BP_CupController_C" _returnvalue "Undefined" 0 0))
  (Variables|Default|SetCupController _returnvalue_2)
  (bind _returnvalue_3 (Game|SpawnActorfromClass "/Game/Blueprints/BP_Cup.BP_Cup_C" _returnvalue "Undefined" 0 0))
  (Variables|Default|SetCupCharacter _returnvalue_3)
  (Pawn|Possess (Variables|Default|GetCupController) (Variables|Default|GetCupCharacter))
  (Audio|PlaySound2D "/Game/Audio/TeaMates_Theme_Song.TeaMates_Theme_Song" 0.5 1.0 0.0 0 0))

(event EventTick
  (params (DeltaSeconds :type Float%20%28single-precision%29))
  (Variables|Default|SetRightVector (* "500.000000,0.000000, 0" DeltaSeconds))
  (Variables|Default|SetUpVector (* "0,-500.000000, 0" DeltaSeconds)))

(event Input|ActionEvents|InputActionResetGame
  (params (Key :type Key%20Structure :default "None"))
  (:Released
    (bind _asgame_mode (Utilities|Casting|CastToGameMode (Game|GetGameMode)))
    (Class|GameMode|RestartGame _asgame_mode)))

(event Input|ActionEvents|InputActionExitGame
  (params (Key :type Key%20Structure :default "None"))
  (:Released
    (Game|QuitGame 0 "Quit" false)))

(event Input|AxisEvents|InputAxisPotRight
  (params (AxisValue :type Float%20%28single-precision%29))
  ;[1 1 1] Pot Movement
  (Pawn|Input|AddMovementInput (Pawn|GetControlledPawn) (Variables|Default|GetRightVector) AxisValue false))

(event Input|AxisEvents|InputAxisCupUp
  (params (AxisValue :type Float%20%28single-precision%29))
  ;[1 1 1] Cup Movement
  (Pawn|Input|AddMovementInput (Variables|Default|GetCupCharacter) (Variables|Default|GetUpVector) AxisValue false))

(event Input|AxisEvents|InputAxisCupRight
  (params (AxisValue :type Float%20%28single-precision%29))
  ;[1 1 1] Cup Movement
  (Pawn|Input|AddMovementInput (Variables|Default|GetCupCharacter) (Variables|Default|GetRightVector) AxisValue false))

(event Input|AxisEvents|InputAxisCupDown
  (params (AxisValue :type Float%20%28single-precision%29))
  ;[1 1 1] Cup Movement
  (Pawn|Input|AddMovementInput (Variables|Default|GetCupCharacter) (Variables|Default|GetUpVector) AxisValue false))

(event Input|AxisEvents|InputAxisCupLeft
  (params (AxisValue :type Float%20%28single-precision%29))
  ;[1 1 1] Cup Movement
  (Pawn|Input|AddMovementInput (Variables|Default|GetCupCharacter) (Variables|Default|GetRightVector) AxisValue false))

(event Input|AxisEvents|InputAxisPotUp
  (params (AxisValue :type Float%20%28single-precision%29))
  ;[1 1 1] Pot Movement
  (Pawn|Input|AddMovementInput (Pawn|GetControlledPawn) (Variables|Default|GetUpVector) AxisValue false))

(event Input|AxisEvents|InputAxisPotDown
  (params (AxisValue :type Float%20%28single-precision%29))
  ;[1 1 1] Pot Movement
  (Pawn|Input|AddMovementInput (Pawn|GetControlledPawn) (Variables|Default|GetUpVector) AxisValue false))

(event Input|AxisEvents|InputAxisPotLeft
  (params (AxisValue :type Float%20%28single-precision%29))
  ;[1 1 1] Pot Movement
  (Pawn|Input|AddMovementInput (Pawn|GetControlledPawn) (Variables|Default|GetRightVector) AxisValue false))

(fn ConstructionScript)

(fn ReduceHealth
  (params (amount :type Integer))
  (bind _output_get (Variables|Default|SetcurrentHealth (- (Variables|Default|GetcurrentHealth) amount)))
  (return _output_get))