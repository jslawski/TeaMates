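; Scoring actor that keeps the current score and shows it as a number on ScoreText.
; OnOrderComplete subtracts the expiry penalty for an expired order and otherwise adds the full MaxScore, with no partial credit or clamping.
; UpdateScore stores each new value and refreshes the text, also running at BeginPlay to show the initial score.
; GetScore exposes the current total.
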(event EventOnOrderComplete
  (params (OrderInfo :type Order%20Info%20Structure))
  (if (.Expired (Utilities|Struct|BreakOrderInfo OrderInfo))
    (CallFunction|UpdateScore (- (Variables|Default|GetcurrentScore) (Variables|Default|GetExpirePenalty)))
    (else
      (CallFunction|UpdateScore (+ (Variables|Default|GetcurrentScore) (Variables|Default|GetMaxScore))))))

(event EventBeginPlay
  (CallFunction|UpdateScore (Variables|Default|GetcurrentScore)))

(fn ConstructionScript)

(fn UpdateScore
  (params (newScore :type Integer))
  (bind _output_get (Variables|Default|SetcurrentScore newScore))
  (Rendering|Components|TextRender|SetText (Variables|Default|GetScoreText) (Utilities|Text|ToText(Integer) _output_get)))

(fn GetScore
  (return (Variables|Default|GetcurrentScore)))