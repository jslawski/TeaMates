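; Spawner actor that repeatedly creates flying things with a configurable angle range, using a referenced FlyingThing as the template for class and transform.
; On BeginPlay it disables that template and starts the DelayTime timeline, which calls Spawn and restarts itself each time it finishes.
; Spawn creates a new actor of the template's class at its location and rotation, then passes it AngleFrom and AngleTo.
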(event EventBeginPlay
  (Variables|/Game/Blueprints/BP_RandomAngleFlyingThing.BP_RandomAngleFlyingThing_C|SetEnabled (Variables|Default|GetFlying%20Thing) false)
  (Timeline|Delay%20Time PlayFromStart
    (:Finished
      (CallFunction|Spawn)
      (Timeline|Delay%20Time PlayFromStart))))

(event Collision|EventActorBeginOverlap
  (params (OtherActor :type Actor%20Object%20Reference)))

(event EventTick
  (params (DeltaSeconds :type Float%20%28single-precision%29)))

(fn ConstructionScript)

(fn Spawn
  (bind _flying_thing (Variables|Default|GetFlying%20Thing))
  (bind _returnvalue (Transformation|GetActorTransform _flying_thing))
  (bind (_location _rotation) (Math|Transform|BreakTransform _returnvalue))
  (bind _returnvalue_2 (Game|SpawnActorfromClass (Utilities|GetClass (Variables|Default|GetFlying%20Thing)) (Math|Transform|MakeTransform _location _rotation "1,1,1") "Undefined" 0 0))
  (Variables|/Game/Blueprints/BP_RandomAngleFlyingThing.BP_RandomAngleFlyingThing_C|SetAngle%20From _returnvalue_2 (Variables|Default|GetAngle%20From))
  (Variables|/Game/Blueprints/BP_RandomAngleFlyingThing.BP_RandomAngleFlyingThing_C|SetAngle%20To _returnvalue_2 (Variables|Default|GetAngle%20To)))