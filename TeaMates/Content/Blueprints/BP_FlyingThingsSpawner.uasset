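; Spawner actor that repeatedly launches BP_FlyingPan actors into the level.
; On BeginPlay the DelayTime timeline acts as a repeating timer, spawning a pan and restarting each time it finishes.
; Each pan takes the referenced FlyingPan actor's location and rotation, randomly offset along world Y within VerticalDisplacementRange.
; An older random-interval Delay loop spawning at the spawner's own transform is left disconnected and never runs.
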(event EventBeginPlay
  (bind _flying_pan (Variables|Default|GetFlying%20Pan))
  (bind _vertical_displacement_range (Variables|Default|GetVertical%20Displacement%20Range))
  (bind _returnvalue (Transformation|GetActorTransform _flying_pan))
  (bind (_location _rotation) (Math|Transform|BreakTransform _returnvalue))
  (Timeline|Delay%20Time PlayFromStart
    (:Finished
      (Game|SpawnActorfromClass "/Game/Blueprints/BP_FlyingPan.BP_FlyingPan_C" (Math|Transform|MakeTransform (+ _location (Math|Vector|MakeVector 0.0 (Math|Random|RandomFloatinRange (* _vertical_displacement_range -1.0) _vertical_displacement_range) 0.0)) _rotation "1,1,1") "Undefined" 0 0)
      (Timeline|Delay%20Time PlayFromStart))))

(event Collision|EventActorBeginOverlap
  (params (OtherActor :type Actor%20Object%20Reference)))

(event EventTick
  (params (DeltaSeconds :type Float%20%28single-precision%29)))

(fn ConstructionScript)