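; BP_Teadrop is a moving tea pickup that comes in four types: black, chai, green and herbal.
; Each Tick it moves by DeltaTransform, or along a random X/Y velocity picked at BeginPlay while the dumping flag is on.
; SetTeaType stores the type and swaps the static mesh to match.
; On any actor overlap it passes one unit of its type through AddTeaMessage, then destroys itself.
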(event EventBeginPlay
  (Variables|Default|SetXDir (Math|Random|RandomFloatinRange 1e+02 2e+02))
  (Variables|Default|SetYDir (Math|Random|RandomFloatinRange 4e+02 5e+02)))

(event EventTick
  (params (DeltaSeconds :type Float%20%28single-precision%29))
  (bind _returnvalue (Transformation|GetActorLocation))
  ;[1 1 1] Teadrop movement
  (if (Variables|Default|GetIsDumping)
    (Transformation|SetActorLocation (+ (* (Math|Vector|MakeVector (Variables|Default|GetXDir) (Variables|Default|GetYDir) 0.0) DeltaSeconds) _returnvalue) false false)
    (else
      (Transformation|SetActorLocation (+ (* (Variables|Default|GetDelta%20Transform) DeltaSeconds) _returnvalue) false false))))

(event Collision|EventActorBeginOverlap
  (params (OtherActor :type Actor%20Object%20Reference))
  (Class|BPTeaHolderInterface|AddTea(Message) OtherActor 1 (Variables|Default|GetTeaType))
  (Actor|DestroyActor))

(fn ConstructionScript)

(fn GetTeaType
  (return (Variables|Default|GetTeaType)))

(fn SetDumping
  (params (newDumping :type Boolean))
  (bind _output_get (Variables|Default|SetIsDumping newDumping))
  (return _output_get))

(fn SetTeaType
  (params (TeaType :type Integer))
  (bind _staticmesh (Variables|Default|GetStaticMesh))
  (bind _output_get (Variables|Default|SetTeaType TeaType))
  (switch int _output_get
    (:Default
      _)
    (:0
      (Components|StaticMesh|SetStaticMesh _staticmesh "/Game/Assets/Meshes/BlackPickup.BlackPickup"))
    (:1
      (Components|StaticMesh|SetStaticMesh _staticmesh "/Game/Assets/Meshes/ChaiPickup.ChaiPickup"))
    (:2
      (Components|StaticMesh|SetStaticMesh _staticmesh "/Game/Assets/Meshes/GreenPickup.GreenPickup"))
    (:3
      (Components|StaticMesh|SetStaticMesh _staticmesh "/Game/Assets/Meshes/HerbalPickup.HerbalPickup")))
  (return 0))