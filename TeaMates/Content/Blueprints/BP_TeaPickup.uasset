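; BP_TeaPickup is a moving tea collectible that refills a BP_Pot on overlap.
; Tick moves it along world +Y at a constant speed without sweeping.
; On overlap with a pot, it sends its tea type and amount, plays a refill sound and destroys itself.
; SetTeaType swaps the static mesh to match one of four teas, while SetRandomTea picks a type at random and clears the CurrentTea text.
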(event Collision|EventActorBeginOverlap
  (params (OtherActor :type Actor%20Object%20Reference))
  (if (Utilities|ClassIsChildOf (Utilities|GetClass OtherActor) "/Game/Blueprints/BP_Pot.BP_Pot_C")
    (Class|BPTeaHolderInterface|AddTea(Message) OtherActor 10 (Variables|Default|GetTeaType))
    (Audio|PlaySound2D "/Game/Audio/Tea_Refill.Tea_Refill" 1.0 1.0 0.0 0 0)
    (Actor|DestroyActor)))

(event EventTick
  (params (DeltaSeconds :type Float%20%28single-precision%29))
  (Transformation|SetActorLocation (+ (* (Math|Vector|MakeVector 0.0 2e+02 0.0) DeltaSeconds) (Transformation|GetActorLocation)) false false))

(fn ConstructionScript)

(fn SetRandomTea
  (CallFunction|SetTeaType (Math|Random|RandomInteger 4))
  (Rendering|Components|TextRender|SetText (Variables|Default|GetCurrentTea) (Utilities|Text|MakeLiteralText "")))

(fn GetTeaMenu
  (return 0))

(fn GetTeaType
  (return (Variables|Default|GetTeaType)))

(fn SetTeaType
  (params (TeaType :type Integer))
  (bind _staticmesh (Variables|Default|GetStaticMesh))
  (bind _output_get (Variables|Default|SetTeaType TeaType))
  (switch int _output_get
    (:Default
      _)
    (:0
      (Components|StaticMesh|SetStaticMesh _staticmesh "/Game/Assets/Meshes/BlackPickup.BlackPickup"))
    (:1
      (Components|StaticMesh|SetStaticMesh _staticmesh "/Game/Assets/Meshes/JasminePickup.JasminePickup"))
    (:2
      (Components|StaticMesh|SetStaticMesh _staticmesh "/Game/Assets/Meshes/GreenPickup.GreenPickup"))
    (:3
      (Components|StaticMesh|SetStaticMesh _staticmesh "/Game/Assets/Meshes/HerbalPickup.HerbalPickup")))
  (return _output_get))