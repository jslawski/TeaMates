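; BackgroundManager is an actor that builds a chain of BP_Background_2 background segments during play.
; On BeginPlay it spawns the first segment at a fixed location and starts a looping 15-second timer.
; Each timer tick spawns a new segment at the previous one's attach point, tracked through LastBackgroundObject.
; Nothing here destroys old segments.
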(event Custom|Event%20Spawn%20Background
  (bind _asbp_background_2 (Utilities|Casting|CastToBP_Background_2 (Variables|Default|GetlastBackgroundObject)))
  (bind _attachposition (Default|GetAttachPoint _asbp_background_2))
  (CallFunction|SpawnBackground (Math|Conversions|ToTransform(Vector) _attachposition)))

(event EventBeginPlay
  (Utilities|FlowControl|Sequence
    (:then_0
      (Utilities|Time|SetTimerbyEvent (delegate Custom|Event%20Spawn%20Background) 15.0 true))
    (:then_1
      (CallFunction|SpawnBackground (Math|Conversions|ToTransform(Vector) "-1100.000000, 0, 0")))))

(event Collision|EventActorBeginOverlap
  (params (OtherActor :type Actor%20Object%20Reference)))

(fn ConstructionScript)

(fn SpawnBackground
  (params (backgroundTransform :type Transform))
  (bind _returnvalue (Game|SpawnActorfromClass "/Game/Blueprints/BP_Background_2.BP_Background_2_C" backgroundTransform "Undefined" 0 0))
  (Variables|Default|SetlastBackgroundObject _returnvalue)
  (return))