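; BP_Cup is a tea cup that tracks how much tea it holds and of what type, showing the amount on its CurrentTea text.
; AddTea increases the total up to a fixed cap, while RemoveTea empties the cup regardless of the amount passed.
; Tea type has its own getter and setter; AddTea ignores its type input because the type-change reset branch is disconnected.
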(event EventBeginPlay
  (Rendering|Components|TextRender|SetText (Variables|Default|GetCurrentTea) (Utilities|Text|ToText(String) (Utilities|String|ToString(Integer) (Variables|Default|GetTotalTea)))))

(event Collision|EventActorBeginOverlap
  (params (OtherActor :type Actor%20Object%20Reference)))

(event EventTick
  (params (DeltaSeconds :type Float%20%28single-precision%29)))

(fn ConstructionScript)

(fn AddTea
  (params (TeaAmount :type Integer) (TeaType :type Integer))
  (Variables|Default|SetTotalTea (+ (Variables|Default|GetTotalTea) TeaAmount))
  (if (> (Variables|Default|GetTotalTea) 30)
    (Variables|Default|SetTotalTea 30))
  (Rendering|Components|TextRender|SetText (Variables|Default|GetCurrentTea) (Utilities|Text|ToText(Integer) (Variables|Default|GetTotalTea)))
  (return (Variables|Default|GetTotalTea)))

(fn GetTeaType
  (return (Variables|Default|GetTeaType)))

(fn GetTotalTea
  (return (Variables|Default|GetTotalTea)))

(fn RemoveTea
  (params (TeaAmount :type Integer))
  (Variables|Default|SetTotalTea 0)
  (Rendering|Components|TextRender|SetText (Variables|Default|GetCurrentTea) (Utilities|Text|ToText(Integer) (Variables|Default|GetTotalTea)))
  (return (Variables|Default|GetTotalTea)))

(fn SetTeaType
  (params (TeaType :type Integer))
  (bind _output_get (Variables|Default|SetTeaType TeaType))
  (return _output_get))