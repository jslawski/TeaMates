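; BP_TeaSpawner is a spawner actor that keeps creating randomized tea pickups at random intervals.
; BeginPlay starts a timer with a random delay between MinTimer and MaxTimer that calls SpawnTea.
; SpawnTea places a BP_TeaPickup at a random X along a fixed world-space line, independent of the spawner's position, and calls SetRandomTea on it.
; It then re-arms the timer with a fresh random delay, so spawning repeats indefinitely.
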(event EventBeginPlay
  (Utilities|Time|SetTimerbyFunctionName 0 "SpawnTea" (Math|Random|RandomFloatinRange (Variables|Default|GetminTimer) (Variables|Default|GetmaxTimer))))

(event Collision|EventActorBeginOverlap
  (params (OtherActor :type Actor%20Object%20Reference)))

(event EventTick
  (params (DeltaSeconds :type Float%20%28single-precision%29)))

(fn ConstructionScript)

(fn SpawnTea
  (bind _returnvalue (Game|SpawnActorfromClass "/Game/Blueprints/BP_TeaPickup.BP_TeaPickup_C" (Math|Transform|MakeTransform (Math|Vector|MakeVector (Math|Random|RandomFloatinRange -1e+03 1e+03) -6e+02 1e+02)) "Undefined" 0 0))
  (Default|SetRandomTea _returnvalue)
  (Utilities|Time|SetTimerbyFunctionName 0 "SpawnTea" (Math|Random|RandomFloatinRange (Variables|Default|GetminTimer) (Variables|Default|GetmaxTimer))))