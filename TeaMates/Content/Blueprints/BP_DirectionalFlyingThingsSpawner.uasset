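; Timed spawner that repeatedly creates flying objects of the same class as its referenced FlyingPan actor.
; On BeginPlay it disables that template actor and starts the DelayTime timeline, which calls Spawn and restarts itself each time it finishes.
; Spawn copies the template's class, location and rotation into a new actor.
; A random vertical displacement calculation is present but unused.
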(event EventBeginPlay
  (Variables|/Game/Blueprints/BP_DirectionalFlyingThing.BP_DirectionalFlyingThing_C|SetEnabled (Variables|Default|GetFlying%20Pan) false)
  (Timeline|Delay%20Time PlayFromStart
    (:Finished
      (CallFunction|Spawn)
      (Timeline|Delay%20Time PlayFromStart))))

(event Collision|EventActorBeginOverlap
  (params (OtherActor :type Actor%20Object%20Reference)))

(event EventTick
  (params (DeltaSeconds :type Float%20%28single-precision%29)))

(fn ConstructionScript)

(fn Spawn
  (bind _flying_pan (Variables|Default|GetFlying%20Pan))
  (bind _returnvalue (Transformation|GetActorTransform _flying_pan))
  (bind (_location _rotation) (Math|Transform|BreakTransform _returnvalue))
  (Game|SpawnActorfromClass (Utilities|GetClass (Variables|Default|GetFlying%20Pan)) (Math|Transform|MakeTransform _location _rotation "1,1,1") "Undefined" 0 0))