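; Actor that launches its physics-driven static mesh in a random horizontal direction with a spin around Z.
; When Enabled, BeginPlay waits briefly, then sets angular velocity from RotationSpeed and linear velocity from MotionSpeed.
; X and Y velocity use the sine and cosine of a random angle expression bounded by AngleFrom and AngleTo.
; A debug print of AngleTo remains; Tick, overlap and construction script are empty.
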(event EventBeginPlay
  (bind _returnvalue (Math|Random|RandomFloat))
  (bind _angle_from (Variables|Default|GetAngle%20From))
  (bind _angle_to (Variables|Default|GetAngle%20To))
  (bind _angle_from_2 (Variables|Default|GetAngle%20From))
  (bind _returnvalue_2 (- _angle_to _angle_from))
  (bind _returnvalue_3 (* _returnvalue _returnvalue_2))
  (bind _returnvalue_4 (+ _angle_from_2 _returnvalue_3))
  (if (Variables|Default|GetEnabled)
    (Utilities|FlowControl|Delay 0.05)
    (Class|PrimitiveComponent|SetPhysicsAngularVelocityinDegrees (Variables|Debug|GetStaticMeshComponent) (Math|Vector|MakeVector 0.0 0.0 (Variables|Default|GetRotation%20Speed)) false "None")
    (Development|PrintString (Utilities|String|ToString(Float) _angle_to))
    (Physics|SetPhysicsLinearVelocity (Variables|Debug|GetStaticMeshComponent) (Math|Vector|MakeVector (* (Variables|Default|GetMotion%20Speed) (Math|Trig|Sin(Degrees) _returnvalue_4)) (* (Variables|Default|GetMotion%20Speed) (Math|Trig|Cos(Degrees) _returnvalue_4)) 0.0) false "None")))

(event Collision|EventActorBeginOverlap
  (params (OtherActor :type Actor%20Object%20Reference)))

(event EventTick
  (params (DeltaSeconds :type Float%20%28single-precision%29)))

(fn ConstructionScript)