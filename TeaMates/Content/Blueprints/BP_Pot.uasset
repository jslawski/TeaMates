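; BP_Pot is a tea pot actor that drips BP_Teadrop actors while the DripTea input is held.
; Press and release open and close a Gate fed by the DripTea axis event, which acts as a per-frame poll.
; Drips fire when key hold time modulo DripCooldown is near zero, so timing depends on frame rate.
; Each drop spawns at the pot's transform composed with OffsetTransform.
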(event EventBeginPlay)

(event Collision|EventActorBeginOverlap
  (params (OtherActor :type Actor%20Object%20Reference)))

(event EventTick
  (params (DeltaSeconds :type Float%20%28single-precision%29)))

(event Input|ActionEvents|InputActionDripTea
  (params (Key :type Key%20Structure :default "None"))
  (:Pressed
    (Utilities|FlowControl|Gate true) ; enters at Open
  )
  (:Released
    (Utilities|FlowControl|Gate true) ; enters at Close
  ))

(event Input|AxisEvents|InputAxisDripTea
  (params (AxisValue :type Float%20%28single-precision%29))
  (Utilities|FlowControl|Gate true
    (:Exit
      (if (Math|Float|NearlyEqual(Float) (Math|Float|%(Float) (Class|PlayerController|GetInputKeyTimeDown (Game|GetPlayerController 0) (stale Input|ActionEvents|InputActionDripTea Key)) (Variables|Default|GetDripCooldown)) 0.0 0.01)
        (Game|SpawnActorfromClass "/Game/Blueprints/BP_Teadrop.BP_Teadrop_C" (Math|Transform|ComposeTransforms (Transformation|GetActorTransform) (Variables|Default|GetOffsetTransform)) "Undefined" 0 0)))))

(fn ConstructionScript)