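; BP_Twitch connects the game to Twitch chat and registers an "order" command for tea orders.
; On BeginPlay it performs a Twitch login, requests the user's own channel feed, stores the chat connection and binds the command.
; The OrderPlaced handler only prints the first parameter, and message and cheer handlers are empty.
; Parameter definitions for tea types exist but are unused.
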(event Custom|OnMessage
  (params (TwitchMessage :type Twitch%20Message%20Structure)))

(event Custom|OnCheer
  (params (TwitchCheer :type Twitch%20Cheer%20Structure)))

(event Custom|OrderPlaced
  (params (Parameters :type Array%20of%20Strings) (Sender :type Twitch%20Message%20Author%20Structure))
  (Development|PrintString (Utilities|String|Append "Order Placed: " (Utilities|Array|Get(acopy) Parameters))))

(event EventBeginPlay
  (bind _credentials (|PerformTwitchLogin)
    (:OnSuccess
      (bind _twitchchat (|RequestFeed (delegate Custom|OnMessage) (delegate Custom|OnCheer) _credentials (.Username (Utilities|Struct|BreakTwitchLoginCredentials _credentials)))
        (:OnSuccessfulLogin
          (Variables|Default|SetChatConnection _twitchchat)
          (Development|PrintString "Successful login!")
          (bind _returnvalue (Class|TwitchPluginBPLibrary|CreateTwitchCommand (Variables|Default|GetChatConnection) (Utilities|Struct|MakeTwitchCommandBinding (Utilities|Struct|MakeTwitchCommand "order" "Put in an order for tea" (Utilities|Array|MakeArray "") false) (EventDispatchers|CreateEvent :!event Custom|OrderPlaced))))
          (Development|PrintString (Utilities|String|Append "Bind Success? " (Utilities|String|ToString(Boolean) _returnvalue))))))))

(event Collision|EventActorBeginOverlap
  (params (OtherActor :type Actor%20Object%20Reference)))

(event EventTick
  (params (DeltaSeconds :type Float%20%28single-precision%29)))

(fn ConstructionScript)

(fn BPTwitchAutoGenFunc
  (params (Parameters :type Array%20of%20Strings) (Sender :type Twitch%20Message%20Author%20Structure))
  (return))